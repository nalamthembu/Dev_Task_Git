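; BP_DialogueCharacter is an interactable character named "Big Head" that bobs in place and takes over the player's view when interacted with.
; Tick adds a sine-of-game-time vertical offset, scaled by speed and height multipliers but not delta time, so the motion depends on frame rate.
; Interact blends the first player controller's view target to this actor.
; GetItemData returns nothing, and no dialogue logic is present.
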(event `self.ReceiveTick`
  (params (DeltaSeconds :type "Float (single-precision)"))
  (`self.K2_AddActorLocalOffset` (* (* (`KismetMathLibrary.Vector_Up`) (`KismetMathLibrary.Sin` (* (`GameplayStatics.GetTimeSeconds`) (`self.SpeedMultiplier`)))) (`self.HeightMultiplier`))))

(fn `GetCharacterName`
  (returns (CharacterName :type Text))
  (return "Big Head"))

(fn `GetItemData`
  (returns (ReturnValue :type "/Game/Blueprints/Data/InventorySystem/BP_InventoryItemData Object Reference"))
  (return null))

(fn `Interact`
  (returns (ItemData :type "/Game/Blueprints/Data/InventorySystem/BP_InventoryItemData Object Reference"))
  (`PlayerController.SetViewTargetWithBlend` (`GameplayStatics.GetPlayerController` 0) self 2.0 "VTBlend_Linear" 0.0 false)
  (return null))

(fn `UserConstructionScript`)