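; Base pickup actor that bobs vertically in the world and hands over its item data when interacted with.
; Tick adds a sine-of-time local Z offset each frame, tuned by speed and height multipliers and not scaled by delta time.
; Interact destroys the actor and returns ItemData if valid, otherwise it prints a missing-data message.
; GetItemData exposes the data without consuming the pickup, while GetCharacterName returns an empty string.
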(event `self.ReceiveTick`
  (params (DeltaSeconds :type "Float (single-precision)"))
  (`self.K2_AddActorLocalOffset` (* (* (`KismetMathLibrary.Vector_Up`) (`KismetMathLibrary.Sin` (* (`GameplayStatics.GetTimeSeconds`) (`self.SpeedMultiplier`)))) (`self.HeightMultiplier`))))

(fn `GetCharacterName`
  (returns (CharacterName :type Text))
  (return ""))

(fn `GetItemData`
  (returns (ReturnValue :type "/Game/Blueprints/Data/InventorySystem/BP_InventoryItemData Object Reference"))
  (return (`self.ItemData`)))

(fn `Interact`
  (returns (ItemData :type "/Game/Blueprints/Data/InventorySystem/BP_InventoryItemData Object Reference"))
  (bind _itemdata (`self.ItemData`)
    (:`then`
      (`self.K2_DestroyActor`)
      (return _itemdata))
    (:`else`
      (`KismetSystemLibrary.PrintString` (`KismetStringLibrary.Concat_StrStr` (`KismetSystemLibrary.GetDisplayName` self) " is missing item data") true true (struct :`R` 1.0 :`G` 0.001 :`A` 1.0)))))

(fn `UserConstructionScript`)