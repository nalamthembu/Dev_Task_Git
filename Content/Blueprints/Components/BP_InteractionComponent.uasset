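; Player interaction component that detects items and dialogue characters under the screen centre and handles interacting with them.
; Each tick a camera-centred sphere trace, more forgiving than a line trace, sets or clears the interactable context.
; Message calls on the target supply item data or a character name for in-range event calls.
; IA_Interact raises an interact event, or looks up the character's ConversationID in DT_Conversations to trigger dialogue.
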(event `self.ReceiveTick`
  (params (DeltaSeconds :type "Float (single-precision)"))
  (bind (_worldposition _worlddirection) (`/Game/Blueprints/Utilities.GetCameraCentrePoint`))
  ; Check if an interactable object is intersecting a spheretrace (Sphere trace has more surface area than a single linetrace
  (bind (_outhit _returnvalue) (`KismetSystemLibrary.SphereTraceSingle` (`/Game/Blueprints/Utilities.GetCameraCentrePoint`) (+ _worldposition (* _worlddirection (`self.MaxInteractionDistance`))) 25.0 "TraceTypeQuery1"))
  (if _returnvalue
    (`/Engine/EditorBlueprintResources/StandardMacros.IsValid` (`self.InteractableContext`)
      (:`Is Not Valid`
        (`self.SetInteractableContext` (`.HitActor` (`GameplayStatics.BreakHitResult` _outhit)))))
    (else
      (`/Engine/EditorBlueprintResources/StandardMacros.IsValid` (`self.InteractableContext`)
        (:`Is Valid`
          (`self.ClearCurrentContext`))))))

(event `EnhancedInput|/Game/Blueprints/Input/Actions/IA_Interact`
  (params (ActionValue :type Boolean) (ElapsedSeconds :type "Float (double-precision)") (TriggeredSeconds :type "Float (double-precision)") (InputAction :type "InputAction Object Reference" :default "/Game/Blueprints/Input/Actions/IA_Interact.IA_Interact"))
  ; Trigger interaction when the player requests it
  (:`Completed`
    (`self.InteractWithContext`)))

(fn `ClearCurrentContext`
  (set `self.InteractableContext` null)
  (`self.OnInteractableOutOfRange`))

(fn `InteractWithContext`
  (bind _interactablecontext (`self.InteractableContext`)
    (:`then`
      (bind _itemdata (message `/Game/Blueprints/Interfaces/BPI_Interactable.Interact` _interactablecontext))
      (`/Engine/EditorBlueprintResources/StandardMacros.IsValid` _itemdata
        (:`Is Valid`
          (`self.OnPlayerInteract` _itemdata)
          (`self.OnInteractableOutOfRange` :!label _label))
        (:`Is Not Valid`
          ; This is just assuming the only thing we'd do with interactables are collect them and talking to them, regardless, find the conversation using the ID from the Data Table
          (bind _asbp_dialogue_character (cast `/Game/Blueprints/Interactables/BP_DialogueCharacter` _interactablecontext))
          (bind _conversationid (`/Game/Blueprints/Interactables/BP_DialogueCharacter.ConversationID` _asbp_dialogue_character))
          (bind _returnvalue (`|GetDataTableRow` "/Game/Blueprints/Data/DataInstances/DT_Conversations.DT_Conversations" _conversationid)
            (:`then`
              (`self.OnPlayerTriggerDialogue` _returnvalue)
              (goto _label))
            (:`RowNotFound`
              (`KismetSystemLibrary.PrintString` (`KismetStringLibrary.Concat_StrStr` "COULD NOT FIND CONVERSATION (" (`KismetStringLibrary.Conv_NameToString` _conversationid) ").") true true (struct :`R` 1.0 :`A` 1.0)))))))
    (:`else`)))

(fn `SetInteractableContext`
  (params (Target :type "Actor Object Reference"))
  (bind _output_get (set `self.InteractableContext` Target))
  (bind _returnvalue (message `/Game/Blueprints/Interfaces/BPI_Interactable.GetItemData` _output_get))
  (`/Engine/EditorBlueprintResources/StandardMacros.IsValid` _returnvalue
    (:`Is Valid`
      (`self.OnInteractableInRange` _returnvalue))
    (:`Is Not Valid`
      ; This will run if the initial data check is invalid meaning the 'target' is probably a character
      (bind _charactername (message `/Game/Blueprints/Interfaces/BPI_Interactable.GetCharacterName` (`local.Target`)))
      (if (not (`KismetTextLibrary.TextIsEmpty` _charactername))
        (`self.OnInRangeOfCharacter` _charactername)))))