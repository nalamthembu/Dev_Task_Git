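; Actor component that manages a player's slot-based inventory, handling item pickup, slot swapping and open/close state.
; It binds to the owner's interaction component so interacted items fill the first free slot with a pickup sound, or signal when capacity is reached.
; Swaps either exchange two slots or move an item into an empty one.
; Event dispatchers announce additions, swaps, full capacity and the IA_Inventory open/close toggle.
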(event `self.ReceiveBeginPlay`
  (bind _returnvalue (`Actor.GetComponentByClass` (`self.GetOwner`) "/Game/Blueprints/Components/BP_InteractionComponent.BP_InteractionComponent_C"))
  (`/Engine/EditorBlueprintResources/StandardMacros.IsValid` _returnvalue
    (:`Is Valid`
      (add `/Game/Blueprints/Components/BP_InteractionComponent.OnPlayerInteract` _returnvalue (delegate `OnPlayerInteract_Event`)))))

(event `OnPlayerInteract_Event`
  (params (ItemData :type "/Game/Blueprints/Data/InventorySystem/BP_InventoryItemData Object Reference"))
  (`self.AddItem` ItemData))

(event `EnhancedInput|/Game/Blueprints/Input/Actions/IA_Inventory`
  (params (ActionValue :type Boolean) (ElapsedSeconds :type "Float (double-precision)") (TriggeredSeconds :type "Float (double-precision)") (InputAction :type "InputAction Object Reference" :default "/Game/Blueprints/Input/Actions/IA_Inventory.IA_Inventory"))
  (:`Triggered`
    (if (`self.IsInventoryOpen`)
      (`self.OnPlayerInventoryClose`)
      (set `self.IsInventoryOpen` false)
      (else
        (`self.OnPlayerInventoryOpen`)
        (set `self.IsInventoryOpen` true)))))

(event `ClosedWithButton`
  (`self.OnPlayerInventoryClose`)
  (set `self.IsInventoryOpen` false))

(fn `AddItem`
  (params (Data :type "/Game/Blueprints/Data/InventorySystem/BP_InventoryItemData Object Reference"))
  (for (_array_element _array_index) (`self.InventorySlots`)
    ; If we find an empty slot, occupy it.
    (if (not (`.isOccupied_5_8764211648FEED148995D89F65AE373F` (break `/Game/Blueprints/Data/InventorySystem/ST_InventorySlot` _array_element)))
      (bind _st_inventoryslot (make `/Game/Blueprints/Data/InventorySystem/ST_InventorySlot` (`local.Data`) true _array_index))
      (`KismetArrayLibrary.Array_Set` (`self.InventorySlots`) _array_index _st_inventoryslot)
      (`GameplayStatics.PlaySound2D` "/Engine/VREditor/Sounds/UI/Object_PickUp.Object_PickUp" 1.0 1.0 0.0 null null)
      (`self.OnAddToInventory` _st_inventoryslot)
      ;[0.5 0.5 0 0.5] Debug
      (`KismetSystemLibrary.PrintString` (`KismetStringLibrary.Concat_StrStr` "Added " (`KismetTextLibrary.Conv_TextToString` (`/Game/Blueprints/Data/InventorySystem/BP_InventoryItemData.ItemName` (`local.Data`)))) true true (struct :`G` 1.0 :`A` 1.0))
      (return)))
  ; All Inventory Slots are occupied
  (`self.OnCapacityReached`)
  (`KismetSystemLibrary.PrintString` "Slots are all occupied" true true (struct :`R` 1.0 :`A` 1.0)))

(fn `SwapItems`
  (params (From :type Integer) (To :type Integer))
  (returns (IsSwappingItems :type Boolean))
  (locals (LocalTempObject :type "/Game/Blueprints/Data/InventorySystem/ST_InventorySlot Structure"))
  (bind _inventoryslots (`self.InventorySlots`))
  (bind _inventoryslots_2 (`self.InventorySlots`))
  (if (`.isOccupied_5_8764211648FEED148995D89F65AE373F` (break `/Game/Blueprints/Data/InventorySystem/ST_InventorySlot` (`|GetArrayItem` (`self.InventorySlots`) (`local.To`))))
    (set `local.LocalTempObject` (`|GetArrayItem` (`self.InventorySlots`) (`local.To`)))
    (`KismetArrayLibrary.Array_Set` _inventoryslots_2 (`local.To`) (`|GetArrayItem` _inventoryslots_2 (`local.From`)))
    (`KismetArrayLibrary.Array_Set` (`self.InventorySlots`) (`local.From`) (`local.LocalTempObject`))
    (else
      (`KismetArrayLibrary.Array_Set` _inventoryslots (`local.To`) (`|GetArrayItem` _inventoryslots (`local.From`)))
      (`KismetArrayLibrary.Array_Set` (`self.InventorySlots`) (`local.From`))))
  (`self.OnInventoryItemSwap` (`local.From`) (`local.To`))
  (return true))