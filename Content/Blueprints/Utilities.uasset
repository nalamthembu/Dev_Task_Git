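; Utility function library of shared helpers for vector math, camera queries, randomness, actor checks and on-screen debug printing.
; Slope angle comes from the movement component's floor normal against up, signed by forward direction so uphill is positive.
; Camera helpers deproject player 0's viewport centre or measure squared camera distance.
; Random helpers cover percentage rolls and uniform unit-circle points; the facing check compares only forward vectors, ignoring positions.
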(fn `ActorIsOfType`
  (params (Actor :type "Actor Object Reference (by ref)") (Class :type "Object Class Reference"))
  (returns (OutActor :type "Actor Object Reference") (ReturnValue :type Boolean))
  (return (`local.Actor`) (`KismetMathLibrary.ClassIsChildOf` (`GameplayStatics.GetObjectClass` Actor) Class)))

(fn `AllAxisNegOne`
  (params (InVector :type "Vector Structure"))
  (returns (Result :type Boolean))
  (return (and (== InVector_X -1.0) (== InVector_Y -1.0) (== InVector_Z -1.0))))

(fn `AngleIsBetween`
  (params (X :type "Float (double-precision)") (A :type "Float (double-precision)") (B :type "Float (double-precision)") (Inclusive :type Boolean))
  (returns (ReturnValue :type Boolean))
  (if Inclusive
    (return (or (and (<= (`local.A`) (`local.X`)) (<= (`local.X`) (`local.B`))) (and (<= (`local.X`) (`local.A`)) (<= (`local.B`) (`local.X`)))))
    (else
      (return (or (and (< (`local.A`) (`local.X`)) (< (`local.X`) (`local.B`))) (and (< (`local.X`) (`local.A`)) (< (`local.B`) (`local.X`))))))))

(fn `AreActorsFacingEachOther`
  (params (A :type "Actor Object Reference") (B :type "Actor Object Reference") (Tolerance :type "Float (double-precision)"))
  (returns (ReturnValue :type Boolean))
  (return (<= (`KismetMathLibrary.Dot_VectorVector` (`Actor.GetActorForwardVector` A) (`Actor.GetActorForwardVector` B)) (* (`KismetMathLibrary.FClamp` Tolerance) -1.0))))

(fn `CalculateAngle`
  (params (a :type "Vector Structure") (b :type "Vector Structure"))
  (returns (Angle :type "Float (double-precision)"))
  (locals (NormalisedA :type "Vector Structure" :default (0.0 0.0 0.0)) (NormalisedB :type "Vector Structure" :default (0.0 0.0 0.0)) (DotProduct :type "Float (double-precision)" :default 0.0))
  (set `local.NormalisedA` (`KismetMathLibrary.Normal` a))
  (set `local.NormalisedB` (`KismetMathLibrary.Normal` b))
  (bind _output_get (set `local.DotProduct` (`KismetMathLibrary.FClamp` (`KismetMathLibrary.Dot_VectorVector` (`local.NormalisedA`) (`local.NormalisedB`)) -1.0)))
  (return (`KismetMathLibrary.DegAcos` _output_get)))

(fn `CalculateChance`
  (params (TargetPercent :type "Float (double-precision)"))
  (returns (Occured :type Boolean))
  (return (<= (`KismetMathLibrary.RandomFloatInRange` 0.0 1.0) (`KismetMathLibrary.SafeDivide` TargetPercent 100.0))))

(fn `CalculateDirection`
  (params (A :type "Vector Structure") (B :type "Vector Structure"))
  (returns (DirectionVector :type "Vector Structure"))
  (return (`KismetMathLibrary.Normal` (- B A))))

(fn `CalculateSlopeAngle`
  (params (CharacterMovementComp :type "CharacterMovementComponent Object Reference"))
  (returns (ReturnValue :type "Float (double-precision)"))
  (locals (SlopeDirection :type "Float (double-precision)") (SurfaceNormal :type "Vector Structure") (SlopeAngle :type "Float (double-precision)" :default 0.0))
  (bind _currentfloor_bblockinghit (break `FindFloorResult` (`CharacterMovementComponent.CurrentFloor` (`local.CharacterMovementComp`))))
  (bind (_currentfloor_bblockinghit_2 _currentfloor_bwalkablefloor _currentfloor_blinetrace _currentfloor_floordist _currentfloor_linedist _currentfloor_hitresult) (break `FindFloorResult` (`CharacterMovementComponent.CurrentFloor` (`local.CharacterMovementComp`))))
  (`|ExecutionSequence`
    (:`then_0`
      (if (not _currentfloor_bblockinghit)
        (return 0.0)))
    (:`then_1`
      ; Get Slope Angle
      (bind _output_get (set `local.SurfaceNormal` (`.Normal` (`GameplayStatics.BreakHitResult` _currentfloor_hitresult))))
      (set `local.SlopeAngle` (`self.CalculateAngle` (`KismetMathLibrary.Vector_Up`) _output_get)))
    (:`then_2`
      ; Calculate Slope Direction
      (bind _output_get_2 (set `local.SlopeDirection` (`KismetMathLibrary.Dot_VectorVector` (`Actor.GetActorForwardVector` (`ActorComponent.GetOwner` (`local.CharacterMovementComp`))) (`local.SurfaceNormal`))))
      ; Flip Slope Angle based on direction (Positive Means Uphill, negative means downhill)
      (if (> _output_get_2 0.0)
        (set `local.SlopeAngle` (* (`local.SlopeAngle`) -1.0))))
    (:`then_3`
      (return (`local.SlopeAngle`)))))

(fn `DebugBool`
  (params (Title :type String) (Bool :type Boolean) (AdditionalDuration :type "Float (double-precision)") (Colour :type "LinearColor Structure"))
  (`KismetSystemLibrary.PrintString` null (`KismetStringLibrary.Concat_StrStr` (`local.Title`) (`KismetStringLibrary.Conv_BoolToString` (`local.Bool`))) true true Colour (+ (`GameplayStatics.GetWorldDeltaSeconds` null) (`local.AdditionalDuration`))))

(fn `DebugFloat`
  (params (Title :type String) (Float :type "Float (double-precision)") (AdditionalDuration :type "Float (double-precision)") (Colour :type "LinearColor Structure"))
  (`KismetSystemLibrary.PrintString` null (`KismetStringLibrary.Concat_StrStr` (`local.Title`) (`KismetStringLibrary.Conv_DoubleToString` (`local.Float`))) true true Colour (+ (`GameplayStatics.GetWorldDeltaSeconds` null) (`local.AdditionalDuration`))))

(fn `DebugString`
  (params (Title :type String) (String :type String) (AdditionalDuration :type "Float (double-precision)") (Colour :type "LinearColor Structure"))
  (`KismetSystemLibrary.PrintString` null (`KismetStringLibrary.Concat_StrStr` (`local.Title`) (`local.String`)) true true Colour (+ (`GameplayStatics.GetWorldDeltaSeconds` null) (`local.AdditionalDuration`))))

(fn `GetCameraCentrePoint`
  (returns (WorldPosition :type "Vector Structure") (WorldDirection :type "Vector Structure"))
  (bind _returnvalue (`GameplayStatics.GetPlayerController` null))
  (bind (_sizex _sizey) (`PlayerController.GetViewportSize` _returnvalue))
  (bind (_worldposition _worlddirection) (`GameplayStatics.DeprojectScreenToWorld` _returnvalue (`KismetMathLibrary.MakeVector2D` (`KismetMathLibrary.Conv_IntToDouble` (/ _sizex 2)) (`KismetMathLibrary.Conv_IntToDouble` (/ _sizey 2)))))
  (return _worldposition _worlddirection))

(fn `GetLocationAheadOfCameraCentrePoint`
  (params (Distance :type "Float (double-precision)"))
  (returns (OutLocation :type "Vector Structure"))
  (bind _returnvalue (`GameplayStatics.GetPlayerController` null))
  (bind (_sizex _sizey) (`PlayerController.GetViewportSize` _returnvalue))
  (bind (_worldposition _worlddirection) (`GameplayStatics.DeprojectScreenToWorld` _returnvalue (`KismetMathLibrary.MakeVector2D` (`KismetMathLibrary.Conv_IntToDouble` (/ _sizex 2)) (`KismetMathLibrary.Conv_IntToDouble` (/ _sizey 2)))))
  (return (+ _worldposition (* _worlddirection (`local.Distance`)))))

(fn `GetRandomPointInUnitCircle`
  (returns (ReturnValue :type "Vector2D Structure"))
  (locals (X :type "Float (double-precision)" :default 0.0) (Y :type "Float (double-precision)" :default 0.0) (Radius :type "Float (double-precision)" :default 0.0) (Angle :type "Float (double-precision)" :default 0.0))
  (set `local.Radius` (`KismetMathLibrary.Sqrt` (`KismetMathLibrary.RandomFloatInRange` 0.0 1.0)))
  (set `local.Angle` (`KismetMathLibrary.RandomFloatInRange` 0.0 (* 2.0 (`KismetMathLibrary.GetPI`))))
  (set `local.X` (* (`local.Radius`) (`KismetMathLibrary.Cos` (`local.Angle`))))
  (set `local.Y` (* (`local.Radius`) (`KismetMathLibrary.Sin` (`local.Angle`))))
  (return (`KismetMathLibrary.MakeVector2D` (`local.X`) (`local.Y`))))

(fn `GetSqrDistanceFromCamera`
  (params (TargetLocation :type "Vector Structure"))
  (returns (ReturnValue :type "Float (double-precision)"))
  (return (`KismetMathLibrary.Vector_DistanceSquared` (`PlayerCameraManager.GetCameraLocation` (`GameplayStatics.GetPlayerCameraManager` null)) TargetLocation)))